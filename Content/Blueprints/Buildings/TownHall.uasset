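; Town Hall building actor that opens a building menu when the player clicks it.
; A click on its Sphere checks the PlayerInstance game instance and proceeds only if the player is not already in a building.
; It creates a BuildingMenu widget, adds it to the viewport, sets its type and the Town Hall level from PlayerInstance, and plays a click sound.
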(event OnClicked(Sphere)
  (params (TouchedComponent :type Primitive%20Component%20Object%20Reference) (ButtonPressed :type Key%20Structure :default "None"))
  (bind _asplayer_instance (Utilities|Casting|CastToPlayerInstance (Game|GetGameInstance)))
  (if (not (Variables|/Game/Saves/PlayerInstance.PlayerInstance_C|GetInBuilding%20? _asplayer_instance))
    (bind _returnvalue (UserInterface|CreateWidget "/Game/UI/BuildingMenu.BuildingMenu_C"))
    (bind _output_get (Variables|Default|SetBuildingMenuRef _returnvalue))
    (UserInterface|Viewport|AddtoViewport _output_get 0)
    (bind _asbuilding_menu (Utilities|Casting|CastToBuildingMenu (Variables|Default|GetBuildingMenuRef)))
    (Variables|/Game/UI/BuildingMenu.BuildingMenu_C|SetBuildingType _asbuilding_menu "Town Hall")
    (bind _asplayer_instance_2 (Utilities|Casting|CastToPlayerInstance (Game|GetGameInstance)))
    (Variables|/Game/UI/BuildingMenu.BuildingMenu_C|SetBuildingLvl (Variables|Default|GetBuildingMenuRef) (Utilities|String|ToString(Integer) (Variables|/Game/Saves/PlayerInstance.PlayerInstance_C|GetTownHalllvl _asplayer_instance_2)))
    (Audio|PlaySound2D "/Game/SFX/Objects/ClickBuilding.ClickBuilding" 1.0 1.0 0.0 0 0)))

(event EventBeginPlay)

(event Collision|EventActorBeginOverlap
  (params (OtherActor :type Actor%20Object%20Reference)))

(event EventTick
  (params (DeltaSeconds :type Float%20%28single-precision%29)))

(fn ConstructionScript)