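; PlayerCharacter is the player's pawn, with world-axis movement and mouse-cursor aiming, as in a top-down game.
; Forward and Right axes add movement along world X and Y, while Tick traces visibility under the cursor and yaws player 0's controlled pawn toward the hit.
; The Debug action opens a DebugMenu widget when InGame is true.
; Death destroys the actor and shows a DeathScreen widget.
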(event EventTick
  (params (DeltaSeconds :type Float%20%28single-precision%29))
  (bind _returnvalue (Game|GetPlayerController 0))
  (bind _returnvalue_2 (Pawn|GetControlledPawn _returnvalue))
  ;[1 1 1] Look at crosshair every ticks
  (Transformation|SetActorRotation _returnvalue_2 (Math|Rotator|MakeRotator 0.0 0.0 (.yaw (Math|Rotator|FindLookatRotation (Transformation|GetActorLocation _returnvalue_2) (.Location (Collision|BreakHitResult (.HitResult (Game|Player|GetHitResultUnderCursorbyChannel _returnvalue "TraceTypeQuery1" true)))))))))

(event Input|ActionEvents|InputActionDebug
  (params (Key :type Key%20Structure :default "None"))
  ;[1 1 1] Open Debug
  (:Pressed
    (if (Variables|Default|GetInGame?)
      (bind _returnvalue (UserInterface|CreateWidget "/Game/UI/DebugMenu.DebugMenu_C"))
      (UserInterface|Viewport|AddtoViewport _returnvalue 0))))

(event Input|AxisEvents|InputAxisForward
  (params (AxisValue :type Float%20%28single-precision%29))
  ;[1 1 1] Mouvements
  (Pawn|Input|AddMovementInput "1.000000, 0, 0" AxisValue false))

(event Input|AxisEvents|InputAxisRight
  (params (AxisValue :type Float%20%28single-precision%29))
  ;[1 1 1] Mouvements
  (Pawn|Input|AddMovementInput "0.000000,1.000000, 0" AxisValue false))

(fn ConstructionScript)

(fn Death
  (Actor|DestroyActor)
  (bind _returnvalue (UserInterface|CreateWidget "/Game/UI/DeathScreen.DeathScreen_C"))
  (UserInterface|Viewport|AddtoViewport _returnvalue 0))